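; Player controller for the hero in a wave survival mode that shows wave announcements and end-of-game screens.
; On BeginPlay, the local controller sets game-only input, starts boss battle music and binds to the survival game state's state-change event.
; Each state change spawns countdown or plain wave text widgets, flagging the last wave.
; Victory or death clears widgets, fades the camera and async-loads the win or lose screen.
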(event `self.ReceiveBeginPlay`
  (if (`self.IsLocalPlayerController`)
    (`WarriorFunctionLibrary.ToogleInputMode` "GameOnly")
    (`GameplayStatics.SpawnSound2D` "/Game/Assets/Sounds/Music/Dungeons_EndBossBattle.Dungeons_EndBossBattle" 1.0 1.0 0.0 null)
    (bind _aswarrior_survial_game_state (cast `WarriorSurvialGameState` (`GameplayStatics.GetGameState`)))
    (bind _output_get (set `self.GameState` _aswarrior_survial_game_state))
    (add `WarriorSurvialGameState.OnCurrentGameStateChange` _output_get (delegate `OnCurrentGameStateChange_事件`))))

(event `OnCurrentGameStateChange_事件`
  (params (CurrentState :type "ESurvivalGameModeState Enum" :default "WaitSpawnNewWave"))
  (bind _gamestate (`self.GameState`))
  (switch `ESurvivalGameModeState` CurrentState
    (:`WaitSpawnNewWave`
      (`self.CreateWaveWidgetWithCountDown` "New Wave Coming In" (`WarriorSurvialGameState.GetSpawnWaitTime` (`self.GameState`))))
    (:`SpawningNewWave`
      (`self.CreateWaveWidgetNoCountDown` (`|FormatText` "Wave {CurrentWaveCount}" (`WarriorSurvialGameState.GetCurrentWaveCount` (`self.GameState`))))
      (if (== (`WarriorSurvialGameState.GetCurrentWaveCount` _gamestate) (`WarriorSurvialGameState.GetTotalWaveToSpawn` _gamestate))
        (`KismetSystemLibrary.Delay` 2.0)
        (`self.CreateWaveWidgetNoCountDown` "Last Wave")))
    (:`WaveComplete`
      (`self.CreateWaveWidgetWithCountDown` (`|FormatText` "Wave {CurrentWaveCount}Completed" (`WarriorSurvialGameState.GetCurrentWaveCount` (`self.GameState`))) (`WarriorSurvialGameState.GetWaveCompletedWaitTime` (`self.GameState`))))
    (:`AllWaveDone`
      (`KismetSystemLibrary.Delay` 1.5)
      (`WidgetLayoutLibrary.RemoveAllWidgets`)
      (`PlayerCameraManager.StartCameraFade` :`self` (`GameplayStatics.GetPlayerCameraManager` 0) :`ToAlpha` 1.0 :`Duration` 2.0)
      (`KismetSystemLibrary.Delay` 1.9)
      (bind _class (`|LoadAssetClass` "/Game/UI/Widgets/Old/GameModeWidget/WBP_WinScreen.WBP_WinScreen_C")
        (:`Completed`
          (bind `_as用户控件` (castclass `UserWidget` _class))
          (bind _returnvalue (`|CreateWidget` `_as用户控件`))
          (`UserWidget.AddToViewport` _returnvalue 0))))
    (:`PlayerDie`
      (`WidgetLayoutLibrary.RemoveAllWidgets`)
      (`PlayerCameraManager.StartCameraFade` :`self` (`GameplayStatics.GetPlayerCameraManager` 0) :`ToAlpha` 1.0 :`Duration` 2.0)
      (`KismetSystemLibrary.Delay` 1.9)
      (bind _class_2 (`|LoadAssetClass` "/Game/UI/Widgets/Old/GameModeWidget/WBP_LoseScreen.WBP_LoseScreen_C")
        (:`Completed`
          (bind `_as用户控件_2` (castclass `UserWidget` _class_2))
          (bind _returnvalue_2 (`|CreateWidget` `_as用户控件_2`))
          (`UserWidget.AddToViewport` _returnvalue_2 0))))))

(fn `CreateWaveWidgetNoCountDown`
  (params (TextContentToDisplay :type Text))
  (bind _returnvalue (`|CreateWidget` "/Game/UI/Widgets/Old/GameModeWidget/WBP_WaveTextNoCountDown.WBP_WaveTextNoCountDown_C"))
  (`UserWidget.AddToPlayerScreen` _returnvalue 0)
  (`TextBlock.SetText` (`/Game/UI/Widgets/Old/GameModeWidget/WBP_WaveTextNoCountDown.TextBlock_WaitText` _returnvalue) (`local.TextContentToDisplay`)))

(fn `CreateWaveWidgetWithCountDown`
  (params (TextContentDisplay :type Text) (InTotalCountDownTime :type "Float (double-precision)"))
  (bind _returnvalue (`|CreateWidget` "/Game/UI/Widgets/Old/GameModeWidget/WBP_WaveTextWithCountDown.WBP_WaveTextWithCountDown_C"))
  (`UserWidget.AddToViewport` _returnvalue 0)
  (`TextBlock.SetText` (`/Game/UI/Widgets/Old/GameModeWidget/WBP_WaveTextWithCountDown.TextBlock_WaitText` _returnvalue) (`local.TextContentDisplay`))
  (`/Game/UI/Widgets/Old/GameModeWidget/WBP_WaveTextWithCountDown.StartCountDown` _returnvalue (`local.InTotalCountDownTime`)))

(fn `UserConstructionScript`)