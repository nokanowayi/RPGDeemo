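; Survival game mode Blueprint that announces wave progress on screen.
; On BeginPlay it binds to its game-state change event and switches on the waiting, spawning and completed wave states.
; Waiting and completed states create countdown text widgets, while spawning shows the wave number without a countdown.
; The final wave also overrides the enemy spawn delay and shows a delayed "Last Wave" banner.
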(event `self.ReceiveBeginPlay`
  (add `self.OnCurrentGameStateChange` (delegate `OnCurrentGameStateChange_事件`)))

(event `OnCurrentGameStateChange_事件` :!signature `self.OnCurrentGameStateChange`
  (params (CurrentState :type "ESurvivalGameModeState Enum" :default "WaitSpawnNewWave"))
  (switch `ESurvivalGameModeState` CurrentState
    (:`WaitSpawnNewWave`
      (`self.CreateWaveWidgetWithCountDown` "New Wave Coming In" (`self.SpawnWaitTime`)))
    (:`SpawningNewWave`
      (`self.CreateWaveWidgetNoCountDown` (`|FormatText` "Wave {CurrentWaveCount}" (`self.CurrentWaveCount`)))
      (if (== (`self.CurrentWaveCount`) (`self.TotalWaveToSpawn`))
        (set `self.SpawnEnemyDelayTime` 4.5)
        (`KismetSystemLibrary.Delay` 2.0)
        (`self.CreateWaveWidgetNoCountDown` "Last Wave")))
    (:`WaveComplete`
      (`self.CreateWaveWidgetWithCountDown` (`|FormatText` "Wave {CurrentWaveCount}Completed" (`self.CurrentWaveCount`)) (`self.WaveCompletedWaitTime`)))))

(fn `CreateWaveWidgetNoCountDown`
  (params (TextContentToDisplay :type Text))
  (bind _returnvalue (`|CreateWidget` "/Game/Widgets/GameModeWidget/WBP_WaveTextNoCountDown.WBP_WaveTextNoCountDown_C"))
  (`UserWidget.AddToPlayerScreen` _returnvalue 0)
  (`TextBlock.SetText` (`/Game/Widgets/GameModeWidget/WBP_WaveTextNoCountDown.TextBlock_WaitText` _returnvalue) (`local.TextContentToDisplay`)))

(fn `CreateWaveWidgetWithCountDown`
  (params (TextContentDisplay :type Text) (InTotalCountDownTime :type "Float (double-precision)"))
  (locals (NewLocalVar :type Text))
  (bind _returnvalue (`|CreateWidget` "/Game/Widgets/GameModeWidget/WBP_WaveTextWithCountDown.WBP_WaveTextWithCountDown_C"))
  (`UserWidget.AddToViewport` _returnvalue 0)
  (`TextBlock.SetText` (`/Game/Widgets/GameModeWidget/WBP_WaveTextWithCountDown.TextBlock_WaitText` _returnvalue) (`local.TextContentDisplay`))
  (`/Game/Widgets/GameModeWidget/WBP_WaveTextWithCountDown.StartCountDown` _returnvalue (`local.InTotalCountDownTime`)))

(fn `UserConstructionScript`)