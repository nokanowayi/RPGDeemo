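; Base gameplay ability for hero Kanata's left light attack, dealing melee damage and building rage.
; It plays an attack montage and waits for melee hit events, each triggering an axe sound cue and a damage spec from equipped weapon damage at the ability level.
; Successful damage sends a hit react event to the target and applies a rage gain effect to the hero.
; Montage completion ends the ability, which removes loose gameplay tags.
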(event `self.K2_ActivateAbility`
  (`AbilityTask_PlayMontageAndWait.CreatePlayMontageAndWaitProxy` "None" (`self.AttackMontage`)
    (:`then`
      (bind (_asynctaskproxy _payload) (`AbilityTask_WaitGameplayEvent.WaitGameplayEvent` (struct :`TagName` "Shared.Event.MeleeHit") null)
        (:`EventReceived`
          (`self.K2_ExecuteGameplayCue` (struct :`TagName` "GameplayCue.Sounds.MeleeHit.Axe"))
          (bind (_eventtag _instigator _target) (break `GameplayEventData` _payload))
          (`self.BP_ApplyGameplaySpecEffectHandleToTarget` _target (`self.MakeHeroDamageEffectSpecHandle` "/Game/Shared/GameplayEffect/GE_Shared_DealDamage.GE_Shared_DealDamage_C" (`HeroCombatComponent.GetHeroCurrentEquippedWeaponDamageAtLevel` (`self.GetHeroCombatComponent`) (`KismetMathLibrary.Conv_IntToDouble` (`self.GetAbilityLevel`))) (struct :`TagName` "Player.SetByCaller.AttackType.Light") 1)
            (:`Successful`
              (`AbilitySystemBlueprintLibrary.SendGameplayEventToActor` _target (struct :`TagName` "Shared.Event.HitReact") _payload)
              (`self.BP_ApplyGameplayEffectToOwner` "/Game/PlayerCharacter/GameplayEffect/GE_Hero_GainRage.GE_Hero_GainRage_C" (`self.GetAbilityLevel`)))))))
    (:`OnCompleted`
      (`self.K2_EndAbility`))))

(event `self.K2_OnEndAbility`
  (params (bWasCancelled :type Boolean))
  (`AbilitySystemBlueprintLibrary.RemoveLooseGameplayTags` (`self.GetAvatarActorFromActorInfo`) (`self.Gameplay Tags`)))