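; Base projectile Blueprint that handles the sound and visual effects of a projectile.
; On BeginPlay it plays a spawn sound and attaches a flying sound that stops when the projectile is destroyed.
; The OnSpawnProjectileHitFX event plays an impact sound and spawns an impact effect at the supplied hit location.
; Each optional asset is validity-checked, but the muzzle effect spawn is disconnected and never runs.
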(event `self.ReceiveBeginPlay`
  (`|ExecutionSequence`
    (:`then_0`
      (bind _projectilespawnsound (`self.ProjectileSpawnSound`)
        (:`then`
          (`GameplayStatics.PlaySoundAtLocation` _projectilespawnsound (`self.K2_GetActorLocation`) (struct) 1.0 1.0 0.0 null null null null))
        (:`else`)))
    (:`then_1`
      (bind _flyingsound (`self.FlyingSound`)
        (:`then`
          (`GameplayStatics.SpawnSoundAttached` _flyingsound (`self.RootComponent`) "None" (0.0 0.0 0.0) (struct) "KeepRelativeOffset" true 1.0 1.0 0.0 null null))
        (:`else`)))
    (:`then_2`
      (bind _projectilemuzzlefx (`self.ProjectileMuzzleFX`)
        (:`then`)
        (:`else`)))))

(event `self.BP_OnSpawnProjectileHitFX`
  (params (HitLocation :type "Vector Structure (by ref)"))
  (`|ExecutionSequence`
    (:`then_0`
      (bind _projectilesound (`self.ProjectileSound`)
        (:`then`
          (`GameplayStatics.PlaySoundAtLocation` _projectilesound HitLocation (struct) 1.0 1.0 0.0 null null null null))
        (:`else`)))
    (:`then_1`
      (bind _projectileimpactfx (`self.ProjectileImpactFX`)
        (:`then`
          (`NiagaraFunctionLibrary.SpawnSystemAtLocation` _projectileimpactfx HitLocation))
        (:`else`)))))

(fn `UserConstructionScript`)